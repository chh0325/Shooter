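; Shooter HUD Blueprint that draws a dynamic crosshair at the center of the screen.
; It caches the player pawn as ShooterCharacterBP on BeginPlay, re-casting in DrawHUD if the reference is invalid.
; Each DrawHUD reads the character's crosshair spread multiplier, scales it by a maximum spread, and draws four directional textures pushed outward from the center by that amount.
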(event `self.ReceiveBeginPlay`
  ;[1 1 1] 判断ShooterCharacter是否有效
  (`/Engine/EditorBlueprintResources/StandardMacros.IsValid` (`self.ShooterCharacter`)
    (:`Is Not Valid`
      (bind _asshooter_character_bp (cast `/Game/_Game/Character/ShooterCharacterBP` (`GameplayStatics.GetPlayerPawn` 0)))
      (set `self.ShooterCharacter` _asshooter_character_bp))))

(event `self.ReceiveDrawHUD`
  (params (SizeX :type Integer) (SizeY :type Integer))
  (bind (_x _y) (`KismetMathLibrary.BreakVector2D` (`self.CrosshairBaseCenter`)))
  (bind (_x_2 _y_2) (`KismetMathLibrary.BreakVector2D` (`self.CrosshairBaseCenter`)))
  (bind (_x_3 _y_3) (`KismetMathLibrary.BreakVector2D` (`self.CrosshairBaseCenter`)))
  (bind (_x_4 _y_4) (`KismetMathLibrary.BreakVector2D` (`self.CrosshairBaseCenter`)))
  (bind (_x_5 _y_5) (`KismetMathLibrary.BreakVector2D` (`self.Crosshair Location`)))
  ;[1 1 1] 设置屏幕中心和十字准线的位置
  (bind _output_get (set `self.Screen Center` (`KismetMathLibrary.MakeVector2D` (`KismetMathLibrary.Conv_IntToDouble` (/ SizeX 2)) (`KismetMathLibrary.Conv_IntToDouble` (/ SizeY 2)))))
  (set `self.Crosshair Location` _output_get)
  ;[1 1 1] 判断ShooterCharacter是否有效
  (`/Engine/EditorBlueprintResources/StandardMacros.IsValid` (`self.ShooterCharacter`)
    (:`Is Valid`
      _)
    (:`Is Not Valid`
      (bind _asshooter_character_bp (cast `/Game/_Game/Character/ShooterCharacterBP` (`GameplayStatics.GetPlayerPawn` 0)))
      (set `self.ShooterCharacter` _asshooter_character_bp)))
  ;[1 1 1] 获取CrosshairSpreadMultiplier
  (set `self.CrosshairSpreadMultiplier` (`ShooterCharacter.GetCrosshairSpreadMultiplier` (`self.ShooterCharacter`)))
  (set `self.CrosshairBaseCenter` (`KismetMathLibrary.MakeVector2D` (- _x_5 (`self.CrosshairHalfWidth`)) (- _y_5 (`self.CrosshairHalfHeight`))))
  (`self.DrawTexture` "/Game/_Game/Assets/Textures/Crosshairs/Crosshair_Quad_9_Bottom.Crosshair_Quad_9_Bottom" _x_3 (+ _y_3 (* (`self.CrosshairSpreadMultiplier`) (`self.CrosshairSpreadMax`))) 64.0 64.0 0.0 0.0 1.0 1.0)
  (`self.DrawTexture` "/Game/_Game/Assets/Textures/Crosshairs/Crosshair_Quad_9_Top.Crosshair_Quad_9_Top" _x_4 (- _y_4 (* (`self.CrosshairSpreadMultiplier`) (`self.CrosshairSpreadMax`))) 64.0 64.0 0.0 0.0 1.0 1.0)
  (`self.DrawTexture` "/Game/_Game/Assets/Textures/Crosshairs/Crosshair_Quad_9_Left.Crosshair_Quad_9_Left" (- _x_2 (* (`self.CrosshairSpreadMultiplier`) (`self.CrosshairSpreadMax`))) _y_2 64.0 64.0 0.0 0.0 1.0 1.0)
  (`self.DrawTexture` "/Game/_Game/Assets/Textures/Crosshairs/Crosshair_Quad_9_Right.Crosshair_Quad_9_Right" (+ _x (* (`self.CrosshairSpreadMultiplier`) (`self.CrosshairSpreadMax`))) _y 64.0 64.0 0.0 0.0 1.0 1.0))

(fn `UserConstructionScript`)